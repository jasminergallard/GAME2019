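; Interactable trigger actor that shows a "wrong item" message when the player interacts with it.
; Overlap enables input and creates a CollectTextPopup, shown only for FirstPersonCharacter, which also opens a gate on the Interact action.
; Through a FlipFlop, every other press displays a WrongItem widget for two seconds before hiding it.
; Ending overlap disables input and hides the popup, leaving the gate open.
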(event `InputAction|Interact`
  (params (Key :type "Key Structure"))
  (:`Pressed`
    (`/Engine/EditorBlueprintResources/StandardMacros.Gate` true :!label _label
      (:`Exit`
        (`/Engine/EditorBlueprintResources/StandardMacros.FlipFlop`
          (:`A`
            (bind _returnvalue (`|CreateWidget` "/Game/Blueprints/Widget/WrongItem.WrongItem_C"))
            (`UserWidget.AddToViewport` _returnvalue 0)
            (`KismetSystemLibrary.Delay` 2.0)
            (`Widget.SetVisibility` _returnvalue "Hidden")))))))

(event `self.ReceiveActorBeginOverlap`
  (params (OtherActor :type "Actor Object Reference"))
  (`self.EnableInput` (`GameplayStatics.GetPlayerController` 0))
  (bind _returnvalue (`|CreateWidget` "/Game/Blueprints/Widget/CollectTextPopup.CollectTextPopup_C"))
  (cast `/Game/FirstPersonBP/Blueprints/FirstPersonCharacter` OtherActor)
  (`UserWidget.AddToViewport` _returnvalue 0)
  (goto _label :!via `Open`))

(event `self.ReceiveActorEndOverlap`
  (params (OtherActor :type "Actor Object Reference"))
  (`self.DisableInput` (`GameplayStatics.GetPlayerController` 0))
  (`WidgetBlueprintLibrary.GetAllWidgetsOfClass` "/Game/Blueprints/Widget/WrongItem.WrongItem_C")
  (`WidgetBlueprintLibrary.GetAllWidgetsOfClass` "/Game/Blueprints/Widget/CollectTextPopup.CollectTextPopup_C")
  (`Widget.SetVisibility` (stale `self.ReceiveActorBeginOverlap` _returnvalue) "Hidden"))

(fn `UserConstructionScript`)