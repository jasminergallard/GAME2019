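; Ghost hazard actor that damages the first-person player when they overlap its Box component.
; A Gate closes after each overlap and reopens after a one-second delay, limiting how often the beep and fixed health loss occur.
; At zero health or below, it shows the HealthNotifications widget, destroys the character and, after a delay, opens the MenuBegin level.
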(event `self.ReceiveHit`
  (params (MyComp :type "PrimitiveComponent Object Reference") (Other :type "Actor Object Reference") (OtherComp :type "PrimitiveComponent Object Reference") (bSelfMoved :type Boolean) (HitLocation :type "Vector Structure") (HitNormal :type "Vector Structure") (NormalImpulse :type "Vector Structure") (Hit :type "HitResult Structure (by ref)")))

(event `self.Box.OnComponentBeginOverlap`
  (params (OverlappedComponent :type "PrimitiveComponent Object Reference") (OtherActor :type "Actor Object Reference") (OtherComp :type "PrimitiveComponent Object Reference") (OtherBodyIndex :type Integer) (bFromSweep :type Boolean) (SweepResult :type "HitResult Structure (by ref)"))
  ;[1 1 1] Damage Player
  (`/Engine/EditorBlueprintResources/StandardMacros.Gate` false :!label _label ; Starts Delay for when player gets hit
    (:`Exit`
      (`|ExecutionSequence`
        (:`then_0`
          (goto _label :!via `Close`))
        (:`then_1`
          (`KismetSystemLibrary.Delay` 1.0) ; Delay after gettting hit
          (goto _label :!via `Open`))
        (:`then_2`
          (if true
            (bind _returnvalue (`GameplayStatics.SpawnSound2D` "/Game/Sound/beep.beep" 1.0 1.0 0.0 null))
            (bind _asfirst_person_character (cast `/Game/FirstPersonBP/Blueprints/FirstPersonCharacter` OtherActor))
            (bind _output_get (set `/Game/FirstPersonBP/Blueprints/FirstPersonCharacter.CurrentHealth` (- (`/Game/FirstPersonBP/Blueprints/FirstPersonCharacter.CurrentHealth` _asfirst_person_character) 25.0) _asfirst_person_character))
            (`/Engine/EditorBlueprintResources/StandardMacros.CompareFloat` _output_get
              (:`>`
                (`KismetSystemLibrary.PrintString` "ALIVE"))
              (:`==`
                (`KismetSystemLibrary.PrintString` "DEAD" :!label _label_2)
                ;[1 1 1] Displays Dead Game Text
                (bind _returnvalue_2 (`|CreateWidget` "/Game/Blueprints/Widget/HealthNotifications.HealthNotifications_C"))
                (`UserWidget.AddToViewport` _returnvalue_2 0)
                ;[1 1 1] Destroys first person character and resets level
                (`self.K2_DestroyActor` _asfirst_person_character)
                (`KismetSystemLibrary.Delay` 3.0)
                (`GameplayStatics.OpenLevel` "MenuBegin"))
              (:`<`
                (goto _label_2)))
            (else
              (`AudioComponent.FadeOut` _returnvalue 0.0 0.0))))))))

(fn `UserConstructionScript`)