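; Level transport actor that lets the player press Interact inside its overlap area to travel to level "3_18_19".
; Overlap enables input, shows the MoveToLevel prompt and opens a gate; leaving disables input and hides the prompt, but never closes the gate.
; Interact passes the gate and a FlipFlop's A branch, disables player input, shows TextDialogue_2, destroys the overlapping FirstPersonCharacter, then loads the level after a short delay.
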(event `self.Box.OnComponentBeginOverlap`
  (params (OverlappedComponent :type "PrimitiveComponent Object Reference") (OtherActor :type "Actor Object Reference") (OtherComp :type "PrimitiveComponent Object Reference") (OtherBodyIndex :type Integer) (bFromSweep :type Boolean) (SweepResult :type "HitResult Structure (by ref)")))

(event `InputAction|Interact`
  (params (Key :type "Key Structure"))
  ;[1 1 1] PRESSING K TO MOVE TO NEXT LEVEL
  (:`Pressed`
    (`/Engine/EditorBlueprintResources/StandardMacros.Gate` true :!label _label
      (:`Exit`
        (`/Engine/EditorBlueprintResources/StandardMacros.FlipFlop`
          (:`A`
            ;;[1 1 1] disbales input
            (`self.DisableInput` (`GameplayStatics.GetPlayerCharacter` 0) (`GameplayStatics.GetPlayerController` 0))
            (bind _asfirst_person_character (cast `/Game/FirstPersonBP/Blueprints/FirstPersonCharacter` (stale `self.ReceiveActorBeginOverlap` OtherActor)))
            (bind _returnvalue (`|CreateWidget` "/Game/Blueprints/Widget/TextDialogue_2.TextDialogue_2_C"))
            (`UserWidget.AddToViewport` _returnvalue 0)
            (`self.K2_DestroyActor` _asfirst_person_character)
            (`KismetSystemLibrary.Delay` 3.0)
            (`GameplayStatics.OpenLevel` "3_18_19")))))))

(event `self.ReceiveActorBeginOverlap`
  (params (OtherActor :type "Actor Object Reference"))
  ;[1 1 1] PRESSING K TO MOVE TO NEXT LEVEL
  (`self.EnableInput` (`GameplayStatics.GetPlayerController` 0))
  (bind _returnvalue (`|CreateWidget` "/Game/Blueprints/Widget/MoveToLevel.MoveToLevel_C"))
  (`UserWidget.AddToViewport` _returnvalue 0)
  (goto _label :!via `Open`))

(event `self.ReceiveActorEndOverlap`
  (params (OtherActor :type "Actor Object Reference"))
  ;[1 1 1] PRESSING K TO MOVE TO NEXT LEVEL
  (`self.DisableInput` (`GameplayStatics.GetPlayerController` 0))
  (`WidgetBlueprintLibrary.GetAllWidgetsOfClass` "/Game/Blueprints/Widget/MoveToLevel.MoveToLevel_C")
  (`Widget.SetVisibility` (stale `self.ReceiveActorBeginOverlap` _returnvalue) "Hidden"))

(fn `UserConstructionScript`)