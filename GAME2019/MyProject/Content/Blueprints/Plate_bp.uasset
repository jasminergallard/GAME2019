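; Collectible plate actor that the first-person character picks up with the Interact input while overlapping it.
; Overlap enables input, shows a CollectTextPopup widget and opens a gate; leaving disables input and hides the popup, but never closes the gate.
; Interact passes through the gate and a FlipFlop, then calls CollectPlate on the overlapping character, destroys the plate and hides the popup.
; Each plate also adds its own Counter widget on BeginPlay.
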(event `InputAction|Interact`
  (params (Key :type "Key Structure"))
  ;[1 1 1] COLLECT PLATE BY PRESSING K
  (:`Pressed`
    (`/Engine/EditorBlueprintResources/StandardMacros.Gate` true :!label _label
      (:`Exit`
        (`/Engine/EditorBlueprintResources/StandardMacros.FlipFlop`
          (:`A`
            (bind _asfirst_person_character (cast `/Game/FirstPersonBP/Blueprints/FirstPersonCharacter` (stale `self.ReceiveActorBeginOverlap` OtherActor)))
            (`/Game/FirstPersonBP/Blueprints/FirstPersonCharacter.CollectPlate` _asfirst_person_character)
            (`self.K2_DestroyActor`)
            (`Widget.SetVisibility` (stale `self.ReceiveActorBeginOverlap` _returnvalue) "Hidden")))))))

(event `self.ReceiveActorBeginOverlap`
  (params (OtherActor :type "Actor Object Reference"))
  ;[1 1 1] COLLECT PLATE BY PRESSING K
  (`self.EnableInput` (`GameplayStatics.GetPlayerController` 0))
  (bind _returnvalue (`|CreateWidget` "/Game/Blueprints/Widget/CollectTextPopup.CollectTextPopup_C"))
  (`UserWidget.AddToViewport` _returnvalue 0)
  (goto _label :!via `Open`))

(event `self.ReceiveActorEndOverlap`
  (params (OtherActor :type "Actor Object Reference"))
  ;[1 1 1] COLLECT PLATE BY PRESSING K
  (`self.DisableInput` (`GameplayStatics.GetPlayerController` 0))
  (`WidgetBlueprintLibrary.GetAllWidgetsOfClass` "/Game/Blueprints/Widget/CollectTextPopup.CollectTextPopup_C")
  (`Widget.SetVisibility` (stale `self.ReceiveActorBeginOverlap` _returnvalue) "Hidden"))

(event `self.ReceiveBeginPlay`
  ;[1 1 1] CREATES WIDGETS
  (bind _returnvalue (`|CreateWidget` "/Game/Blueprints/Widget/Counter.Counter_C"))
  (`UserWidget.AddToViewport` _returnvalue 0))

(fn `UserConstructionScript`)