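; Door actor that, in its live logic, acts as an end-game trigger for the first-person character.
; On overlap it casts the other actor to FirstPersonCharacter and calls its EndGame, followed by a one-second delay that leads nowhere.
; Key-count checks, the open-door widget, input gating and self-destruction are disconnected leftovers.
; DoorOpen is an empty function, with its Door1open level sequence player also left unwired.
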(event `self.ReceiveActorBeginOverlap`
  (params (OtherActor :type "Actor Object Reference"))
  (bind _asfirst_person_character (cast `/Game/FirstPersonBP/Blueprints/FirstPersonCharacter` OtherActor))
  (`/Game/FirstPersonBP/Blueprints/FirstPersonCharacter.EndGame` _asfirst_person_character)
  (`KismetSystemLibrary.Delay` 1.0))

(event `InputAction|Interact`
  (params (Key :type "Key Structure")))

(event `self.ReceiveActorEndOverlap`
  (params (OtherActor :type "Actor Object Reference")))

(fn `DoorOpen`)

(fn `UserConstructionScript`)