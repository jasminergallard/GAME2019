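; Bear_BP is a collectible bear actor that the player picks up with the Interact input while overlapping it.
; Beginning an overlap enables input, shows a CollectTextPopup and opens a gate; ending it disables input and hides the popup, leaving the gate open.
; Interact passes through the gate and a FlipFlop's A branch to call CollectBear on the overlapping FirstPersonCharacter, then destroys the bear.
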(event `InputAction|Interact`
  (params (Key :type "Key Structure"))
  ;[1 1 1] Press k to pick up
  (:`Pressed`
    (`/Engine/EditorBlueprintResources/StandardMacros.Gate` true :!label _label
      (:`Exit`
        (`/Engine/EditorBlueprintResources/StandardMacros.FlipFlop`
          (:`A`
            (bind _asfirst_person_character (cast `/Game/FirstPersonBP/Blueprints/FirstPersonCharacter` (stale `self.ReceiveActorBeginOverlap` OtherActor)))
            (`/Game/FirstPersonBP/Blueprints/FirstPersonCharacter.CollectBear` _asfirst_person_character)
            (`self.K2_DestroyActor`)))))))

(event `self.ReceiveActorBeginOverlap`
  (params (OtherActor :type "Actor Object Reference"))
  ;[1 1 1] Press k to pick up
  (`self.EnableInput` (`GameplayStatics.GetPlayerController` 0))
  (bind _returnvalue (`|CreateWidget` "/Game/Blueprints/Widget/CollectTextPopup.CollectTextPopup_C"))
  (`UserWidget.AddToViewport` _returnvalue 0)
  (goto _label :!via `Open`))

(event `self.ReceiveActorEndOverlap`
  (params (OtherActor :type "Actor Object Reference"))
  ;[1 1 1] Press k to pick up
  (`self.DisableInput` null)
  (`WidgetBlueprintLibrary.GetAllWidgetsOfClass` "/Game/Blueprints/Widget/CollectTextPopup.CollectTextPopup_C")
  (`Widget.SetVisibility` (stale `self.ReceiveActorBeginOverlap` _returnvalue) "Hidden"))

(fn `UserConstructionScript`)