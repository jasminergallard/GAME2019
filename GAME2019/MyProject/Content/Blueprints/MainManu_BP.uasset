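; Main menu actor that shows a menu widget on BeginPlay and handles leaving it for the StartLevel map.
; BeginPlay also enables input on the actor and opens a gate for the Interact action.
; The first press disables player character input, hides top-level MainMenu widgets and destroys the actor.
; The one-second delay and level load are wired after DestroyActor, so they likely never complete.
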(event `self.ReceiveBeginPlay`
  (bind _returnvalue (`|CreateWidget` "/Game/Blueprints/Widget/MainMenu.MainMenu_C"))
  (`UserWidget.AddToViewport` _returnvalue 0)
  (`self.EnableInput` (`GameplayStatics.GetPlayerController` 0))
  (goto _label :!via `Open`))

(event `InputAction|Interact`
  (params (Key :type "Key Structure"))
  (:`Pressed`
    (`/Engine/EditorBlueprintResources/StandardMacros.Gate` true :!label _label
      (:`Exit`
        (`/Engine/EditorBlueprintResources/StandardMacros.FlipFlop`
          (:`A`
            (`self.DisableInput` (`GameplayStatics.GetPlayerCharacter` 0) (`GameplayStatics.GetPlayerController` 0))
            (bind _foundwidgets (`WidgetBlueprintLibrary.GetAllWidgetsOfClass` "/Game/Blueprints/Widget/MainMenu.MainMenu_C"))
            (`Widget.SetVisibility` _foundwidgets "Hidden")
            (`self.K2_DestroyActor`)
            (`KismetSystemLibrary.Delay` 1.0)
            (`GameplayStatics.OpenLevel` "StartLevel")))))))

(event `self.ReceiveActorBeginOverlap`
  (params (OtherActor :type "Actor Object Reference")))

(fn `UserConstructionScript`)